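; Player-controllable tank Blueprint that sets up C++ turret, barrel and track components and routes input to them.
; The construction script assigns meshes and a track physical material; BeginPlay hands component references to TankAiming and TankMovement.
; Input drives tracks directly or through TankMovement's move and turn intents, and fires through TankAiming.
; Camera aim splits yaw onto an azimuth gimbal and pitch onto the spring arm.
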(event EventBeginPlay
  (Class|TankAimingComponent|InitialiseBarrelTurret (Variables|Default|GetTankAiming) (Variables|Default|GetTankTurretCPP) (Variables|Default|GetTankBarrelCPP))
  (Class|TankMovementComponent|Initialise (Variables|Default|GetTankMovement) (Variables|Default|GetLeftTrackCPP) (Variables|Default|GetRightTrackCPP)))

(event Collision|EventActorBeginOverlap
  (params (OtherActor :type Actor%20Object%20Reference)))

(event EventTick
  (params (DeltaSeconds :type Float%20%28single-precision%29)))

(event Input|ActionEvents|InputActionFireProjectile
  (params (Key :type Key%20Structure :default "None"))
  ;[1 1 1] Firing Projectile
  (:Pressed
    (Class|TankAimingComponent|Fire (Variables|Default|GetTankAiming))))

(event Input|AxisEvents|InputAxisLeftTrackThrottle
  (params (AxisValue :type Float%20%28single-precision%29))
  (Class|TankTrack|SetThrottle (Variables|Default|GetLeftTrackCPP) AxisValue))

(event Input|AxisEvents|InputAxisAimElevation
  (params (AxisValue :type Float%20%28single-precision%29))
  ;[1 1 1] Camera Input Binding
  (Transformation|AddLocalRotation (Variables|Default|GetSpringArm) (Math|Rotator|MakeRotator 0.0 AxisValue 0.0) false false))

(event Input|AxisEvents|InputAxisAimAzimuth
  (params (AxisValue :type Float%20%28single-precision%29))
  ;[1 1 1] Camera Input Binding
  (Transformation|AddLocalRotation (Variables|Default|GetAzimuth%20Gimble) (Math|Rotator|MakeRotator 0.0 0.0 AxisValue) false false))

(event Input|AxisEvents|InputAxisRightTrackThrottle
  (params (AxisValue :type Float%20%28single-precision%29))
  (Class|TankTrack|SetThrottle (Variables|Default|GetRightTrackCPP) AxisValue))

(event Input|AxisEvents|InputAxisMoveForward
  (params (AxisValue :type Float%20%28single-precision%29))
  (Class|TankMovementComponent|IntendMoveForward (Variables|Default|GetTankMovement) AxisValue))

(event Input|AxisEvents|InputAxisTurnRight
  (params (AxisValue :type Float%20%28single-precision%29))
  (Class|TankMovementComponent|IntendTurnRight (Variables|Default|GetTankMovement) AxisValue))

(fn ConstructionScript
  (Components|StaticMesh|SetStaticMesh (Variables|Default|GetTankTurretCPP) "/Game/TankModel/tank_fbx_Turret.tank_fbx_Turret")
  (Components|StaticMesh|SetStaticMesh (Variables|Default|GetTankBarrelCPP) "/Game/TankModel/tank_fbx_Barrel.tank_fbx_Barrel")
  (Components|StaticMesh|SetStaticMesh (Variables|Default|GetLeftTrackCPP) "/Game/TankModel/tank_fbx_Track.tank_fbx_Track")
  (Components|StaticMesh|SetStaticMesh (Variables|Default|GetRightTrackCPP) "/Game/TankModel/tank_fbx_Track.tank_fbx_Track")
  (Class|PrimitiveComponent|SetPhysMaterialOverride (Variables|Default|GetLeftTrackCPP) "/Game/TankModel/Track.Track")
  (Class|PrimitiveComponent|SetPhysMaterialOverride (Variables|Default|GetRightTrackCPP) "/Game/TankModel/Track.Track"))